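; First-person demo character for previewing the sci-fi impact, tracer and decal effects by shooting at surfaces.
; WASD timelines feed movement input from camera vectors, mouse axes drive look, and Space jumps.
; Left click line-traces from GunPoint, spawning the tracer, an impact effect on blocking hits, and a random fading decal regardless of hit.
; R steps a looping MultiGate through alien, energy and technology impact systems, each paired with a tracer colour.
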(event `Key|SpaceBar`
  (params (Key :type "Key Structure"))
  (:`Pressed`
    (`self.Jump`)))

(event `Key|W`
  (params (Key :type "Key Structure"))
  (:`Pressed`
    (`Timeline|Timeline_0` :!via `PlayFromStart` :!label _label
      (:`Update`
        (`self.AddMovementInput` (* (`SceneComponent.GetForwardVector` (`self.Camera`)) 10.0)))))
  (:`Released`
    (goto _label :!via `Stop`)))

(event `Key|A`
  (params (Key :type "Key Structure"))
  (:`Pressed`
    (`Timeline|Timeline_1` :!via `PlayFromStart` :!label _label_2
      (:`Update`
        (`self.AddMovementInput` (* (`SceneComponent.GetRightVector` (`self.Camera`)) -10.0)))))
  (:`Released`
    (goto _label_2 :!via `Stop`)))

(event `Key|S`
  (params (Key :type "Key Structure"))
  (:`Pressed`
    (`Timeline|Timeline_2` :!via `PlayFromStart` :!label _label_3
      (:`Update`
        (`self.AddMovementInput` (* (`SceneComponent.GetForwardVector` (`self.Camera`)) -10.0)))))
  (:`Released`
    (goto _label_3 :!via `Stop`)))

(event `Key|D`
  (params (Key :type "Key Structure"))
  (:`Pressed`
    (`Timeline|Timeline_3` :!via `PlayFromStart` :!label _label_4
      (:`Update`
        (`self.AddMovementInput` (* (`SceneComponent.GetRightVector` (`self.Camera`)) 10.0)))))
  (:`Released`
    (goto _label_4 :!via `Stop`)))

(event `InputAxisKey|MouseX`
  (params (AxisValue :type "Float (single-precision)"))
  (`self.AddControllerYawInput` AxisValue))

(event `InputAxisKey|MouseY`
  (params (AxisValue :type "Float (single-precision)"))
  (`self.AddControllerPitchInput` (* AxisValue -1.0)))

(event `Key|LeftMouseButton`
  (params (Key :type "Key Structure"))
  (bind _gunpoint (`self.GunPoint`))
  (bind _returnvalue (`SceneComponent.K2_GetComponentLocation` _gunpoint))
  (bind _returnvalue_2 (`SceneComponent.K2_GetComponentRotation` _gunpoint))
  (:`Pressed`
    (bind _outhit (`KismetSystemLibrary.LineTraceSingle` :`Start` _returnvalue :`End` (+ _returnvalue (* (`KismetMathLibrary.GetForwardVector` _returnvalue_2) (`KismetMathLibrary.Conv_DoubleToVector` 20000.0))) :`TraceChannel` "TraceTypeQuery1" :`DrawTime` 2.0))
    (bind (_bblockinghit _binitialoverlap _time _distance _location _impactpoint _normal) (`GameplayStatics.BreakHitResult` _outhit))
    (if _bblockinghit
      (`NiagaraFunctionLibrary.SpawnSystemAtLocation` (`self.Impact`) _location))
    (`NiagaraFunctionLibrary.SpawnSystemAtLocation` (`self.Tracer`) _returnvalue _returnvalue_2)
    (bind (_returnvalue_roll _returnvalue_pitch _returnvalue_yaw) (`KismetMathLibrary.BreakRotator` (`KismetMathLibrary.Conv_VectorToRotator` _normal)))
    (bind _returnvalue_3 (`GameplayStatics.SpawnDecalAtLocation` (`KismetArrayLibrary.Array_Random` (`self.Decal Material`)) (16.0 32.0 32.0) _location (`KismetMathLibrary.MakeRotator` (`KismetMathLibrary.RandomFloatInRange` 0.0 360.0) (+ _returnvalue_pitch 180.0) _returnvalue_yaw) 10.0))
    (`DecalComponent.SetFadeOut` _returnvalue_3 5.0 5.0 true)))

(event `Key|R`
  (params (Key :type "Key Structure"))
  (:`Pressed`
    (`|MultiGate` false true 1
      (:`Out 0`
        (set `self.Impact` "/Game/SciFi_Impacts/FX/NS_Alien_Impact_1.NS_Alien_Impact_1")
        (set `self.Tracer` "/Game/SciFi_Impacts/FX/NS_Tracer_Green.NS_Tracer_Green"))
      (:`Out 1`
        (set `self.Impact` "/Game/SciFi_Impacts/FX/NS_Alien_Impact_2.NS_Alien_Impact_2")
        (set `self.Tracer` "/Game/SciFi_Impacts/FX/NS_Tracer_Red.NS_Tracer_Red"))
      (:`Out 2`
        (set `self.Impact` "/Game/SciFi_Impacts/FX/NS_Alien_Impact_3.NS_Alien_Impact_3")
        (set `self.Tracer` "/Game/SciFi_Impacts/FX/NS_Tracer_GreenOrange.NS_Tracer_GreenOrange"))
      (:`Out 3`
        (set `self.Impact` "/Game/SciFi_Impacts/FX/NS_Alien_Impact_4.NS_Alien_Impact_4")
        (set `self.Tracer` "/Game/SciFi_Impacts/FX/NS_Tracer_YellowGreen.NS_Tracer_YellowGreen"))
      (:`Out 4`
        (set `self.Impact` "/Game/SciFi_Impacts/FX/NS_Alien_Impact_5.NS_Alien_Impact_5")
        (set `self.Tracer` "/Game/SciFi_Impacts/FX/NS_Tracer_GreenOrange.NS_Tracer_GreenOrange"))
      (:`Out 5`
        (set `self.Impact` "/Game/SciFi_Impacts/FX/NS_Alien_Impact_6.NS_Alien_Impact_6")
        (set `self.Tracer` "/Game/SciFi_Impacts/FX/NS_Tracer_Green.NS_Tracer_Green"))
      (:`Out 6`
        (set `self.Impact` "/Game/SciFi_Impacts/FX/NS_Alien_Impact_7.NS_Alien_Impact_7")
        (set `self.Tracer` "/Game/SciFi_Impacts/FX/NS_Tracer_BluePurple.NS_Tracer_BluePurple"))
      (:`Out 7`
        (set `self.Impact` "/Game/SciFi_Impacts/FX/NS_Alien_Impact_8.NS_Alien_Impact_8")
        (set `self.Tracer` "/Game/SciFi_Impacts/FX/NS_Tracer_Pink.NS_Tracer_Pink"))
      (:`Out 8`
        (set `self.Impact` "/Game/SciFi_Impacts/FX/NS_Alien_Impact_9.NS_Alien_Impact_9")
        (set `self.Tracer` "/Game/SciFi_Impacts/FX/NS_Tracer_TealGreen.NS_Tracer_TealGreen"))
      (:`Out 9`
        (set `self.Impact` "/Game/SciFi_Impacts/FX/NS_Energy_Impact_1.NS_Energy_Impact_1")
        (set `self.Tracer` "/Game/SciFi_Impacts/FX/NS_Tracer_Blue.NS_Tracer_Blue"))
      (:`Out 10`
        (set `self.Impact` "/Game/SciFi_Impacts/FX/NS_Energy_Impact_2.NS_Energy_Impact_2")
        (set `self.Tracer` "/Game/SciFi_Impacts/FX/NS_Tracer_Purple.NS_Tracer_Purple"))
      (:`Out 11`
        (set `self.Impact` "/Game/SciFi_Impacts/FX/NS_Energy_Impact_3.NS_Energy_Impact_3")
        (set `self.Tracer` "/Game/SciFi_Impacts/FX/NS_Tracer_Yellow.NS_Tracer_Yellow"))
      (:`Out 12`
        (set `self.Impact` "/Game/SciFi_Impacts/FX/NS_Energy_Impact_4.NS_Energy_Impact_4")
        (set `self.Tracer` "/Game/SciFi_Impacts/FX/NS_Tracer_Yellow.NS_Tracer_Yellow"))
      (:`Out 13`
        (set `self.Impact` "/Game/SciFi_Impacts/FX/NS_Energy_Impact_5.NS_Energy_Impact_5")
        (set `self.Tracer` "/Game/SciFi_Impacts/FX/NS_Tracer_Blue.NS_Tracer_Blue"))
      (:`Out 14`
        (set `self.Impact` "/Game/SciFi_Impacts/FX/NS_Energy_Impact_6.NS_Energy_Impact_6")
        (set `self.Tracer` "/Game/SciFi_Impacts/FX/NS_Tracer_YellowOrange.NS_Tracer_YellowOrange"))
      (:`Out 15`
        (set `self.Impact` "/Game/SciFi_Impacts/FX/NS_Energy_Impact_7.NS_Energy_Impact_7")
        (set `self.Tracer` "/Game/SciFi_Impacts/FX/NS_Tracer_RedBlue.NS_Tracer_RedBlue"))
      (:`Out 16`
        (set `self.Impact` "/Game/SciFi_Impacts/FX/NS_Energy_Impact_8.NS_Energy_Impact_8")
        (set `self.Tracer` "/Game/SciFi_Impacts/FX/NS_Tracer_Orange.NS_Tracer_Orange"))
      (:`Out 17`
        (set `self.Impact` "/Game/SciFi_Impacts/FX/NS_Energy_Impact_9.NS_Energy_Impact_9")
        (set `self.Tracer` "/Game/SciFi_Impacts/FX/NS_Tracer_BlueYellow.NS_Tracer_BlueYellow"))
      (:`Out 18`
        (set `self.Impact` "/Game/SciFi_Impacts/FX/NS_Technology_Impact_1.NS_Technology_Impact_1")
        (set `self.Tracer` "/Game/SciFi_Impacts/FX/NS_Tracer_Blue.NS_Tracer_Blue"))
      (:`Out 19`
        (set `self.Impact` "/Game/SciFi_Impacts/FX/NS_Technology_Impact_2.NS_Technology_Impact_2")
        (set `self.Tracer` "/Game/SciFi_Impacts/FX/NS_Tracer_BlueYellow.NS_Tracer_BlueYellow"))
      (:`Out 20`
        (set `self.Impact` "/Game/SciFi_Impacts/FX/NS_Technology_Impact_3.NS_Technology_Impact_3")
        (set `self.Tracer` "/Game/SciFi_Impacts/FX/NS_Tracer_BlueGreen.NS_Tracer_BlueGreen"))
      (:`Out 21`
        (set `self.Impact` "/Game/SciFi_Impacts/FX/NS_Technology_Impact_4.NS_Technology_Impact_4")
        (set `self.Tracer` "/Game/SciFi_Impacts/FX/NS_Tracer_BluePurple.NS_Tracer_BluePurple"))
      (:`Out 22`
        (set `self.Impact` "/Game/SciFi_Impacts/FX/NS_Technology_Impact_5.NS_Technology_Impact_5")
        (set `self.Tracer` "/Game/SciFi_Impacts/FX/NS_Tracer_BlueYellow.NS_Tracer_BlueYellow"))
      (:`Out 23`
        (set `self.Impact` "/Game/SciFi_Impacts/FX/NS_Technology_Impact_6.NS_Technology_Impact_6")
        (set `self.Tracer` "/Game/SciFi_Impacts/FX/NS_Tracer_BluePurple.NS_Tracer_BluePurple"))
      (:`Out 24`
        (set `self.Impact` "/Game/SciFi_Impacts/FX/NS_Technology_Impact_7.NS_Technology_Impact_7")
        (set `self.Tracer` "/Game/SciFi_Impacts/FX/NS_Tracer_RedBlue.NS_Tracer_RedBlue"))
      (:`Out 25`
        (set `self.Impact` "/Game/SciFi_Impacts/FX/NS_Technology_Impact_8.NS_Technology_Impact_8")
        (set `self.Tracer` "/Game/SciFi_Impacts/FX/NS_Tracer_Purple.NS_Tracer_Purple"))
      (:`Out 26`
        (set `self.Impact` "/Game/SciFi_Impacts/FX/NS_Technology_Impact_9.NS_Technology_Impact_9")
        (set `self.Tracer` "/Game/SciFi_Impacts/FX/NS_Tracer_Pink.NS_Tracer_Pink")))))

(fn `UserConstructionScript`)