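; Configurable sci-fi weapon Blueprint covering five guns: handgun, assault, SMG, shotgun and sniper.
; SetWeaponMesh picks body and magazine meshes by WeaponTypes, attaching the magazine to the "Mag" socket.
; SkinTypes chooses default, color, texture or blend materials, using per-weapon helpers for the first three and dynamic instances for custom parameters.
; This setup logic sits disconnected from the empty Construction Script, so it never runs.
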(fn `ColorMaterials`
  (switch `/Game/Assets/Scifi_Weapon_Vol01/Blueprints/EN_Weapons` (`self.WeaponTypes`)
    (:`NewEnumerator0`
      (set `self.ColorMaterial` "/Game/Assets/Scifi_Weapon_Vol01/Material/MI_Katta_Pistol_01a_ColorInst.MI_Katta_Pistol_01a_ColorInst"))
    (:`NewEnumerator1`
      (set `self.ColorMaterial` "/Game/Assets/Scifi_Weapon_Vol01/Material/MI_SSK-80_Assault_01a_ColorInst.MI_SSK-80_Assault_01a_ColorInst"))
    (:`NewEnumerator2`
      (set `self.ColorMaterial` "/Game/Assets/Scifi_Weapon_Vol01/Material/MI_Devore_SMG_01a_ColorInst.MI_Devore_SMG_01a_ColorInst"))
    (:`NewEnumerator3`
      (set `self.ColorMaterial` "/Game/Assets/Scifi_Weapon_Vol01/Material/MI_MoxT20_Shotgun_01a_ColorInst.MI_MoxT20_Shotgun_01a_ColorInst"))
    (:`NewEnumerator4`
      (set `self.ColorMaterial` "/Game/Assets/Scifi_Weapon_Vol01/Material/MI_DRT-20_Sniper_01a_ColorInst.MI_DRT-20_Sniper_01a_ColorInst"))))

(fn `DefaultMaterials`
  (switch `/Game/Assets/Scifi_Weapon_Vol01/Blueprints/EN_Weapons` (`self.WeaponTypes`)
    (:`NewEnumerator0`
      (set `self.DefaultMaterial` "/Game/Assets/Scifi_Weapon_Vol01/Material/MI_Katta_Pistol_01a_Inst.MI_Katta_Pistol_01a_Inst"))
    (:`NewEnumerator1`
      (set `self.DefaultMaterial` "/Game/Assets/Scifi_Weapon_Vol01/Material/MI_SSK-80_Assault_01a_Inst.MI_SSK-80_Assault_01a_Inst"))
    (:`NewEnumerator2`
      (set `self.DefaultMaterial` "/Game/Assets/Scifi_Weapon_Vol01/Material/MI_Devore_SMG_01a_Inst.MI_Devore_SMG_01a_Inst"))
    (:`NewEnumerator3`
      (set `self.DefaultMaterial` "/Game/Assets/Scifi_Weapon_Vol01/Material/MI_MoxT20_Shotgun_01a_Inst.MI_MoxT20_Shotgun_01a_Inst"))
    (:`NewEnumerator4`
      (set `self.DefaultMaterial` "/Game/Assets/Scifi_Weapon_Vol01/Material/MI_DRT-20_Sniper_01a_Inst.MI_DRT-20_Sniper_01a_Inst"))))

(fn `SetWeaponMesh`
  (`SkinnedMeshComponent.SetSkinnedAssetAndUpdate` (`self.WeaponMesh`) (select `/Game/Assets/Scifi_Weapon_Vol01/Blueprints/EN_Weapons` (`self.WeaponTypes`) :`NewEnumerator0` "/Game/Assets/Scifi_Weapon_Vol01/Mesh/Katta_Pistol/SK_Katta_Handgun_X_01a.SK_Katta_Handgun_X_01a" :`NewEnumerator1` "/Game/Assets/Scifi_Weapon_Vol01/Mesh/SSK-80_Assault/SK_SSK-80_Assault_X_01a.SK_SSK-80_Assault_X_01a" :`NewEnumerator2` "/Game/Assets/Scifi_Weapon_Vol01/Mesh/Devore_SMG/SK_Devore_SMG_X_01a.SK_Devore_SMG_X_01a" :`NewEnumerator3` "/Game/Assets/Scifi_Weapon_Vol01/Mesh/Mox_T20_Shotgun/SK_MoxT20_Shotgun_X_01a.SK_MoxT20_Shotgun_X_01a" :`NewEnumerator4` "/Game/Assets/Scifi_Weapon_Vol01/Mesh/DRT-20_Sniper/SK_DTR-20_Sniper_X_01a.SK_DTR-20_Sniper_X_01a" :!type "SkeletalMesh Object Reference") true)
  (`StaticMeshComponent.SetStaticMesh` (`self.MagMesh`) (select `/Game/Assets/Scifi_Weapon_Vol01/Blueprints/EN_Weapons` (`self.WeaponTypes`) :`NewEnumerator0` "/Game/Assets/Scifi_Weapon_Vol01/Mesh/Katta_Pistol/SM_Katta_Mag.SM_Katta_Mag" :`NewEnumerator1` "/Game/Assets/Scifi_Weapon_Vol01/Mesh/SSK-80_Assault/SM_SSK-80_Mag_01a.SM_SSK-80_Mag_01a" :`NewEnumerator2` "/Game/Assets/Scifi_Weapon_Vol01/Mesh/Devore_SMG/SM_Devore_Mag_01a.SM_Devore_Mag_01a" :`NewEnumerator3` "/Game/Assets/Scifi_Weapon_Vol01/Mesh/Mox_T20_Shotgun/SM_MoxT20_Mag_01a.SM_MoxT20_Mag_01a" :`NewEnumerator4` "/Game/Assets/Scifi_Weapon_Vol01/Mesh/DRT-20_Sniper/SM_DTR-20_Mag_01a.SM_DTR-20_Mag_01a" :!type "StaticMesh Object Reference"))
  (`SceneComponent.K2_AttachToComponent` (`self.MagMesh`) (`self.WeaponMesh`) "Mag" "KeepRelative" "KeepRelative" "KeepRelative" true))

(fn `TextureMaterials`
  (switch `/Game/Assets/Scifi_Weapon_Vol01/Blueprints/EN_Weapons` (`self.WeaponTypes`)
    (:`NewEnumerator0`
      (set `self.TextureMaterial` "/Game/Assets/Scifi_Weapon_Vol01/Material/MI_Katta_Pistol_01a_TextureInst.MI_Katta_Pistol_01a_TextureInst"))
    (:`NewEnumerator1`
      (set `self.TextureMaterial` "/Game/Assets/Scifi_Weapon_Vol01/Material/MI_SSK-80_Assault_01a_TextureInst.MI_SSK-80_Assault_01a_TextureInst"))
    (:`NewEnumerator2`
      (set `self.TextureMaterial` "/Game/Assets/Scifi_Weapon_Vol01/Material/MI_Devore_SMG_01a_TextureInst.MI_Devore_SMG_01a_TextureInst"))
    (:`NewEnumerator3`
      (set `self.TextureMaterial` "/Game/Assets/Scifi_Weapon_Vol01/Material/MI_MoxT20_Shotgun_01a_TextureInst.MI_MoxT20_Shotgun_01a_TextureInst"))
    (:`NewEnumerator4`
      (set `self.TextureMaterial` "/Game/Assets/Scifi_Weapon_Vol01/Material/MI_DRT-20_Sniper_01a_TextureInst.MI_DRT-20_Sniper_01a_TextureInst"))))

(fn `UserConstructionScript`)