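; Weapon pickup actor that gives the first-person character one of five sci-fi guns on contact.
; The construction script sets the skeletal mesh from the SelectWeapon choice.
; A timeline spins the mesh by adding its value to the current yaw each update, replaying after a short delay.
; Overlapping the sphere copies SelectWeapon to the character's WeaponType, calls ChangeWeapon, then destroys the pickup.
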(event `self.ReceiveBeginPlay`
  (bind _weaponmesh (`self.WeaponMesh`))
  (bind (_relativerotation_roll _relativerotation_pitch _relativerotation_yaw) (`KismetMathLibrary.BreakRotator` (`SceneComponent.RelativeRotation` _weaponmesh)))
  (bind (_direction _value) (`Timeline|RotationTImeline` :!label _label)
    (:`Update`
      (`SceneComponent.K2_SetRelativeRotation` _weaponmesh (`KismetMathLibrary.MakeRotator` _relativerotation_roll _relativerotation_pitch (+ _value _relativerotation_yaw)) false false))
    (:`Finished`
      (`KismetSystemLibrary.Delay` 0.2)
      (goto _label :!via `PlayFromStart`))))

(event `self.Sphere.OnComponentBeginOverlap`
  (params (OverlappedComponent :type "PrimitiveComponent Object Reference") (OtherActor :type "Actor Object Reference") (OtherComp :type "PrimitiveComponent Object Reference") (OtherBodyIndex :type Integer) (bFromSweep :type Boolean) (SweepResult :type "HitResult Structure (by ref)"))
  (bind _asfirst_person_character (cast `/Game/Assets/Scifi_Weapon_Vol01/Unreal_FPS_Arms/FirstPersonBP/Blueprints/FirstPersonCharacter` OtherActor))
  (set `/Game/Assets/Scifi_Weapon_Vol01/Unreal_FPS_Arms/FirstPersonBP/Blueprints/FirstPersonCharacter.WeaponType` (`self.SelectWeapon`) _asfirst_person_character)
  (`/Game/Assets/Scifi_Weapon_Vol01/Unreal_FPS_Arms/FirstPersonBP/Blueprints/FirstPersonCharacter.ChangeWeapon` _asfirst_person_character)
  (`self.K2_DestroyActor`))

(fn `UserConstructionScript`
  (switch `/Game/Assets/Scifi_Weapon_Vol01/Blueprints/EN_Weapons` (`self.SelectWeapon`)
    (:`NewEnumerator0`
      (`SkinnedMeshComponent.SetSkinnedAssetAndUpdate` (`self.WeaponMesh`) "/Game/Assets/Scifi_Weapon_Vol01/Mesh/Katta_Pistol/SK_Katta_Handgun_X_01a.SK_Katta_Handgun_X_01a" true))
    (:`NewEnumerator1`
      (`SkinnedMeshComponent.SetSkinnedAssetAndUpdate` (`self.WeaponMesh`) "/Game/Assets/Scifi_Weapon_Vol01/Mesh/SSK-80_Assault/SK_SSK-80_Assault_X_01a.SK_SSK-80_Assault_X_01a" true))
    (:`NewEnumerator2`
      (`SkinnedMeshComponent.SetSkinnedAssetAndUpdate` (`self.WeaponMesh`) "/Game/Assets/Scifi_Weapon_Vol01/Mesh/Devore_SMG/SK_Devore_SMG_X_01a.SK_Devore_SMG_X_01a" true))
    (:`NewEnumerator3`
      (`SkinnedMeshComponent.SetSkinnedAssetAndUpdate` (`self.WeaponMesh`) "/Game/Assets/Scifi_Weapon_Vol01/Mesh/Mox_T20_Shotgun/SK_MoxT20_Shotgun_X_01a.SK_MoxT20_Shotgun_X_01a" true))
    (:`NewEnumerator4`
      (`SkinnedMeshComponent.SetSkinnedAssetAndUpdate` (`self.WeaponMesh`) "/Game/Assets/Scifi_Weapon_Vol01/Mesh/DRT-20_Sniper/SK_DTR-20_Sniper_X_01a.SK_DTR-20_Sniper_X_01a" true))))