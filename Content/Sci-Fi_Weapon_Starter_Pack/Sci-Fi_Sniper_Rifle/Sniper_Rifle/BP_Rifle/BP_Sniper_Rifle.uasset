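; BP_Sniper_Rifle is a sci-fi sniper rifle actor with a camera-fed scope display.
; Each tick it applies the display zoom FOV to a scene capture and, per CameraONOFF, either routes it to a render target with the camera-on scope material or clears both.
; When DisplayRotate is set, Tick also replays the display freeze animation on the scope mesh every frame.
; The construction script toggles front scope glass visibility from ScopeGlassHide.
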(event `self.ReceiveTick`
  (params (DeltaSeconds :type "Float (single-precision)"))
  (bind _rifledisplaycapture (`self.RifleDisplayCapture`))
  (bind _sk_scope (`self.SK_Scope`))
  (`|ExecutionSequence`
    (:`then_0`
      ;[1 1 1] v1 Display
      (set `SceneCaptureComponent2D.FOVAngle` (`self.Fov_ZoomDisplay`) (`self.RifleDisplayCapture`))
      (if (`self.CameraON/OFF`)
        (`PrimitiveComponent.SetMaterial` _sk_scope 0 "/Game/Sci-Fi_Weapon_Starter_Pack/Sci-Fi_Sniper_Rifle/Sniper_Rifle/Material_Rifle/MI_Scope_On_Camera.MI_Scope_On_Camera")
        (set `SceneCaptureComponent2D.TextureTarget` "/Game/Sci-Fi_Weapon_Starter_Pack/Sci-Fi_Sniper_Rifle/Sniper_Rifle/Material_Rifle/Source/Texture/RT_Camera.RT_Camera" _rifledisplaycapture)
        (else
          (`PrimitiveComponent.SetMaterial` _sk_scope 0 null)
          (set `SceneCaptureComponent2D.TextureTarget` null _rifledisplaycapture))))
    (:`then_1`
      ;[1 1 1] Anim Freeze display
      (if (`self.DisplayRotate?`)
        (`SkeletalMeshComponent.PlayAnimation` (`self.SK_Scope`) "/Game/Sci-Fi_Weapon_Starter_Pack/Sci-Fi_Sniper_Rifle/Sniper_Rifle/Anim_Rifle/Anim_Scope/Anim_Freeze_Display.Anim_Freeze_Display" false)))))

(event `self.ReceiveBeginPlay`)

(fn `UserConstructionScript`
  (bind _sm_glass_front (`self.SM_Glass_Front`))
  (if (`self.ScopeGlassHide?`)
    (`SceneComponent.SetVisibility` _sm_glass_front false false)
    (else
      (`SceneComponent.SetVisibility` _sm_glass_front true false))))